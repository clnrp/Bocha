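; MyBall_OBP is a physics ball that adjusts its own rolling speed and reports when it stops.
; Each tick it adds the GameInstance_OBP Reduce rate, scaled by delta time and velocity sign, to X velocity, then Y, which changes only while X is moving.
; Once speed falls to a small threshold, it latches Stopped, sets BallStopped on the game instance and prints a debug message.
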(event EventBeginPlay)

(event EventTick
  (params (DeltaSeconds :type Float%20%28single-precision%29))
  (Utilities|FlowControl|Sequence
    (:then_0
      (bind _asgame_instance_obp (Utilities|Casting|CastToGameInstance_OBP (Game|GetGameInstance)))
      (bind _returnvalue (Physics|GetPhysicsLinearVelocity (Variables|Default|GetStaticMesh) "None"))
      (Variables|Default|SetTime (+ DeltaSeconds (Variables|Default|GetTime)))
      (Math|Float|CompareFloat (Math|Float|Absolute(Float) (.x _returnvalue)) 0.0
        (:>
          (Physics|SetPhysicsLinearVelocity (Variables|Default|GetStaticMesh) (Math|Vector|MakeVector (* (* (Variables|/Game/Blueprints/GameInstance_OBP.GameInstance_OBP_C|GetReduce _asgame_instance_obp) DeltaSeconds) (Math|Float|Sign(Float) (.x _returnvalue))) 0.0 0.0) true "None")
          (Math|Float|CompareFloat (Math|Float|Absolute(Float) (.y _returnvalue)) 0.0
            (:>
              (Physics|SetPhysicsLinearVelocity (Variables|Default|GetStaticMesh) (Math|Vector|MakeVector 0.0 (* (* (Variables|/Game/Blueprints/GameInstance_OBP.GameInstance_OBP_C|GetReduce _asgame_instance_obp) DeltaSeconds) (Math|Float|Sign(Float) (.y _returnvalue))) 0.0) true "None"))))))
    (:then_1
      (if (not (Variables|Default|GetStopped))
        (bind _returnvalue_2 (Physics|GetPhysicsLinearVelocity (Variables|Default|GetStaticMesh) "None"))
        (Math|Float|CompareFloat (Math|Vector|VectorLength _returnvalue_2) 1.0
          (:==
            _)
          (:<
            _))
        (bind _asgame_instance_obp_2 (Utilities|Casting|CastToGameInstance_OBP (Game|GetGameInstance)))
        (Variables|/Game/Blueprints/GameInstance_OBP.GameInstance_OBP_C|SetBallStopped _asgame_instance_obp_2 true)
        (Variables|Default|SetStopped true)
        (Development|PrintString "Parou")))))

(fn ConstructionScript)
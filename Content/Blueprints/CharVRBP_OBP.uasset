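; VR player character that throws a ball in turns with an adversary, using the right motion controller trigger.
; Holding the trigger shows a held ball whose velocity is tracked each Tick; releasing spawns MyBall_OBP, launched horizontally along the controller's forward at that speed.
; GameInstance_OBP holds the turn flags, polled every Tick and updated on throw.
; A Teleport function shifts position along negative world X.
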(event EventBeginPlay)

(event EventTick
  (params (DeltaSeconds :type Float%20%28single-precision%29))
  (bind _ball (Variables|Default|GetBall))
  (bind _returnvalue (Transformation|GetWorldLocation _ball))
  (bind _asgame_instance_obp (Utilities|Casting|CastToGameInstance_OBP (Game|GetGameInstance)))
  (Variables|Default|SetAdversary (Variables|/Game/Blueprints/GameInstance_OBP.GameInstance_OBP_C|GetAdversary _asgame_instance_obp))
  (Variables|Default|SetBallStopped (Variables|/Game/Blueprints/GameInstance_OBP.GameInstance_OBP_C|GetBallStopped _asgame_instance_obp))
  (if (Rendering|IsVisible (Variables|Default|GetBall))
    (bind _output_get (Variables|Default|SetBallSpeed (/ (- _returnvalue (Variables|Default|GetBallPosition)) DeltaSeconds)))
    (Variables|Default|SetBallPosition _returnvalue)))

(event Input|KeyboardEvents|MotionControllerRightTrigger
  (params (Key :type Key%20Structure))
  (bind _motioncontroller (Variables|Default|GetMotionController))
  (bind _ballspeed (Variables|Default|GetBallSpeed))
  (bind _ball (Variables|Default|GetBall))
  (bind _returnvalue (Math|Vector|VectorLength _ballspeed))
  (bind _returnvalue_2 (Math|Vector|GetForwardVector _motioncontroller))
  (bind _returnvalue_3 (Math|Float|Absolute(Float) _returnvalue))
  (bind _returnvalue_4 (Math|Vector|Normalize _returnvalue_2))
  (bind _returnvalue_5 (* _returnvalue_3 1.0))
  (:Pressed
    (if (and (not (Variables|Default|GetAdversary)) (Variables|Default|GetBallStopped))
      (Rendering|SetVisibility _ball true false)))
  (:Released
    (if (and (not (Variables|Default|GetAdversary)) (Variables|Default|GetBallStopped))
      (Rendering|SetVisibility _ball false false)
      (bind _returnvalue_6 (Game|SpawnActorfromClass "/Game/Blueprints/MyBall_OBP.MyBall_OBP_C" (Math|Transform|MakeTransform (Variables|Default|GetBallPosition) "0, 0, 0" "0.500000,0.500000,0.500000") "Undefined" 0 0))
      (Physics|SetPhysicsLinearVelocity (Variables|/Game/Blueprints/MyBall_OBP.MyBall_OBP_C|GetStaticMesh _returnvalue_6) (Math|Vector|MakeVector (* (.x _returnvalue_4) _returnvalue_5) (* (.y _returnvalue_4) _returnvalue_5) 0.0) true "None")
      (bind _asgame_instance_obp (Utilities|Casting|CastToGameInstance_OBP (Game|GetGameInstance)))
      (Variables|/Game/Blueprints/GameInstance_OBP.GameInstance_OBP_C|SetAdversary _asgame_instance_obp true)
      (Variables|/Game/Blueprints/GameInstance_OBP.GameInstance_OBP_C|SetBallStopped _asgame_instance_obp false))))

(fn ConstructionScript)

(fn Teleport
  (params (self2 :type Actor%20Object%20Reference))
  (bind _returnvalue (Transformation|GetActorLocation self2))
  (Transformation|Teleport (Math|Vector|MakeVector (+ (.x _returnvalue) -1.5e+02) (+ (.y _returnvalue) 0.0) (.z _returnvalue)) "0, 0, 0"))
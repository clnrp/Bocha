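; Points is an actor that displays two ball counts, MyBalls and AdBalls, in the Bocha game.
; Every Tick it casts the game instance to BochaGameInstanceBP and polls those values, setting the MyPoints and AdPoints text only where it differs.
; The AdPoints check is nested inside the MyPoints change branch, so AdPoints refreshes only on a tick when MyPoints also changes.
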(event EventBeginPlay)

(event Collision|EventActorBeginOverlap
  (params (OtherActor :type Actor%20Object%20Reference)))

(event EventTick
  (params (DeltaSeconds :type Float%20%28single-precision%29))
  (bind _mypoints (Variables|Default|GetMyPoints))
  (bind _adpoints (Variables|Default|GetAdPoints))
  (bind _asbocha_game_instance_bp (Utilities|Casting|CastToBochaGameInstanceBP (Game|GetGameInstance)))
  (if (Utilities|Enum|NotEqual(Enum) (Variables|/Script/Engine.TextRenderComponent|GetText _mypoints) (Utilities|Text|ToText(Integer) (Variables|/Script/Bocha.BochaGameInstance|GetMyBalls _asbocha_game_instance_bp)))
    (Rendering|Components|TextRender|SetText _mypoints (Utilities|Text|ToText(Integer) (Variables|/Script/Bocha.BochaGameInstance|GetMyBalls _asbocha_game_instance_bp)))
    (if (Utilities|Enum|NotEqual(Enum) (Utilities|Text|ToText(Integer) (Variables|/Script/Bocha.BochaGameInstance|GetAdBalls _asbocha_game_instance_bp)) (Variables|/Script/Engine.TextRenderComponent|GetText _adpoints))
      (Rendering|Components|TextRender|SetText _adpoints (Utilities|Text|ToText(Integer) (Variables|/Script/Bocha.BochaGameInstance|GetAdBalls _asbocha_game_instance_bp))))))

(fn ConstructionScript)